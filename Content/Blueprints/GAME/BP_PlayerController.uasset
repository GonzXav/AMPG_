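; BP_PlayerController is a player controller that handles mouse-look camera rotation.
; On BeginPlay it adds its Enhanced Input mapping context to the local player subsystem.
; The IA_Look action drives yaw and pitch input scaled by MouseSensitivity, with the vertical axis inverted.
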(event Input|EnhancedActionEvents|EnhancedInputActionIA_Look
  (params (ActionValue :type Vector%202D%20Structure) (ElapsedSeconds :type Float%20%28double-precision%29) (TriggeredSeconds :type Float%20%28double-precision%29) (InputAction :type Input%20Action%20Object%20Reference :default "/Game/Blueprints/GAME/Input/Actions/IA_Look.IA_Look"))
  (bind _mousesensitivity (Variables|Default|GetMouseSensitivity))
  ;[1 1 1] Camera Rotation
  (:Triggered
    (Class|PlayerController|AddYawInput (* (.x ActionValue) _mousesensitivity))
    (Class|PlayerController|AddPitchInput (* (* (.y ActionValue) _mousesensitivity) -1.0))))

(event EventBeginPlay
  (bind _self self)
  (bind _returnvalue (PlayerController|LocalPlayerSubsystems|GetEnhancedInputLocalPlayerSubsystem _self))
  (Utilities|IsValid _returnvalue
    (:Is%20Valid
      (Input|AddMappingContext _returnvalue "/Game/Blueprints/GAME/Input/IMC_PlayerControllerMappingContext.IMC_PlayerControllerMappingContext" 0 "(bIgnoreAllPressedKeysUntilRelease=True,bForceImmediately=False)"))))

(event EventTick
  (params (DeltaSeconds :type Float%20%28single-precision%29)))

(fn ConstructionScript)