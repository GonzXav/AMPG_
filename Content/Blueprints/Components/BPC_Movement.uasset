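; Movement component that gives the player character stamina-limited sprinting and crouching by changing the CharacterMovement max walk speed.
; Looping timers drain stamina while sprinting, stopping when it runs out or the player stops moving, then refill it after a retriggerable delay.
; Crouching blocks and cancels sprinting, then calls the owning character to shorten or lengthen its capsule.
; The character reference is passed in through Initialize, which also applies the default walk speed.
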(event Custom|StartSprinting
  (if (not (Variables|Default|GetIsCrouching))
    (if (and (> (Variables|Default|GetCurrentStamina) (Variables|Default|GetMinStamina)) (CallFunction|IsPlayerMoving))
      (Utilities|Time|ClearTimerbyFunctionName 0 "RegenerateStamina")
      (CallFunction|SetMaxWalkSpeed (Variables|Default|GetSprintSpeed))
      (Utilities|Time|SetTimerbyFunctionName 0 "SprintTimer" 0.1 true))))

(event Custom|SprintTimer
  (Variables|Default|SetCurrentStamina (Math|Float|Clamp(Float) (- (Variables|Default|GetCurrentStamina) (Variables|Default|GetStaminaDepletionAmount)) (Variables|Default|GetMinStamina) (Variables|Default|GetMaxStamina)))
  (if (<= (Variables|Default|GetCurrentStamina) (Variables|Default|GetMinStamina))
    (CallFunction|StopSprinting :!label _label)
    (elif (not (and (> (Variables|Default|GetCurrentStamina) (Variables|Default|GetMinStamina)) (CallFunction|IsPlayerMoving)))
      (goto _label))))

(event Custom|StopSprinting
  (Utilities|Time|ClearTimerbyFunctionName 0 "SprintTimer")
  (CallFunction|SetMaxWalkSpeed (Variables|Default|GetWalkSpeed))
  (Utilities|FlowControl|RetriggerableDelay 5.0)
  (if (not (Class|KismetSystemLibrary|IsTimerActive 0 "SprintTimer"))
    (Utilities|Time|SetTimerbyFunctionName 0 "RegenerateStamina" 0.03 true)))

(event Custom|RegenerateStamina
  (bind _output_get (Variables|Default|SetCurrentStamina (Math|Float|Clamp(Float) (+ (Variables|Default|GetCurrentStamina) (Variables|Default|GetStaminaReplenishAmount)) (Variables|Default|GetMinStamina) (Variables|Default|GetMaxStamina))))
  (if (>= _output_get (Variables|Default|GetMaxStamina))
    (Utilities|Time|ClearTimerbyFunctionName 0 "RegenerateStamina")))

(event Custom|BeginCrouch
  ;[1 1 1] Crouch
  (Variables|Default|SetIsCrouching true)
  (Utilities|Time|ClearTimerbyFunctionName 0 "SprintTimer")
  (CallFunction|SetMaxWalkSpeed (Variables|Default|GetCrouchWalkSpeed))
  (Default|ShortenPlayerCapsule (Variables|Default|GetBP_Character_REF)))

(event Custom|EndCrouch
  ;[1 1 1] Crouch
  (Variables|Default|SetIsCrouching false)
  (CallFunction|SetMaxWalkSpeed (Variables|Default|GetWalkSpeed))
  (Default|LengthenPlayerCapsule (Variables|Default|GetBP_Character_REF)))

(event EventBeginPlay)

(event EventTick
  (params (DeltaSeconds :type Float%20%28single-precision%29)))

(fn Initialize
  (params (BP_Player_REF :type BP%20Player%20Character%20Object%20Reference))
  (Variables|Default|SetBP_Character_REF BP_Player_REF)
  (CallFunction|SetMaxWalkSpeed (Variables|Default|GetWalkSpeed)))

(fn SetMaxWalkSpeed
  (params (MaxWalkSpeed :type Float%20%28single-precision%29))
  (Variables|/Script/Engine.CharacterMovementComponent|SetMaxWalkSpeed (Variables|/Script/Engine.Character|GetCharacterMovement (Variables|Default|GetBP_Character_REF)) MaxWalkSpeed))

(fn IsPlayerMoving
  (return (> (Math|Vector|VectorLength (Transformation|GetVelocity (Variables|Default|GetBP_Character_REF))) 1e+01)))