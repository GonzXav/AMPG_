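; BP_InteractableDoor is an interactable door actor that toggles open and closed when its interaction event fires.
; On opening, the dot product of the player-to-door direction and the actor's forward vector picks the swing sign, up to 90 degrees either way.
; A timeline drives the door's yaw and reverses to close.
; CanInteract blocks retriggering until the timeline finishes and a short delay updates IsOpen from its direction.
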(event Custom|Open/CloseDoor
  (bind _self self)
  (if (Variables|Default|GetCanInteract)
    (Variables|Default|SetCanInteract false)
    (if (not (Variables|Default|GetIsOpen))
      (Variables|Default|SetDotProduct (Math|Vector|DotProduct (Math|Vector|Normalize (- (Transformation|GetActorLocation _self) (Transformation|GetActorLocation (Variables|Default|GetBP_Player_REF)))) (Transformation|GetActorForwardVector _self)))
      (bind (_direction _alpha) (Timeline|DoorSwing_TL PlayFromStart)
        (:Update
          (Transformation|SetRelativeRotation (Variables|Default|GetDoor) (Math|Rotator|MakeRotator 0.0 0.0 (Math|Float|Lerp 0.0 (select (>= (Variables|Default|GetDotProduct) 0.0) 9e+01 -9e+01) _alpha)) false false))
        (:Finished
          (Utilities|FlowControl|Delay 0.25)
          (switch Utilities|FlowControl|Switch|SwitchonETimelineDirection _direction
            (:Forward
              (Variables|Default|SetIsOpen true))
            (:Backward
              (Variables|Default|SetIsOpen false)))
          (Variables|Default|SetCanInteract true)))
      (else
        (Timeline|DoorSwing_TL ReverseFromEnd)))))

(event EventBeginPlay
  (|CallParentFunction) ; This node is disabled and will not be called.\nDrag off pins to build functionality.
)

(event Collision|EventActorBeginOverlap
  (params (OtherActor :type Actor%20Object%20Reference))
  (|CallParentFunction OtherActor) ; This node is disabled and will not be called.\nDrag off pins to build functionality.
)

(event EventTick
  (params (DeltaSeconds :type Float%20%28single-precision%29))
  (|CallParentFunction DeltaSeconds) ; This node is disabled and will not be called.\nDrag off pins to build functionality.
)

(event EventBeginInteration
  (CallFunction|Open/CloseDoor))

(fn ConstructionScript
  (|CallParentFunction))